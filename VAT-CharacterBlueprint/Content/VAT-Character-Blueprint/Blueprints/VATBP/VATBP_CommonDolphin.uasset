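; Playable or AI-driven dolphin that uses a vertex animation texture (VAT) state-machine material, applied to its mesh as a dynamic instance on BeginPlay.
; When the AI flag is set, Tick moves it toward a Destination actor without pathfinding and interpolates its pitch to face it.
; Axis inputs handle mouse look and movement, blending control and actor rotation with that same Destination-facing pitch.
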(event `AI`
  (bind _returnvalue (`self.K2_GetActorRotation`))
  ;[1 1 1] Navigation
  (bind _returnvalue_2 (`GameplayStatics.GetActorOfClass` (`GameplayStatics.GetObjectClass` (`self.Destination`))))
  (`AITask_MoveTo.AIMoveTo` (`AIBlueprintHelperLibrary.GetAIController` self) (`self.K2_GetActorLocation` _returnvalue_2) _returnvalue_2 -1.0 "Default" "Default" false false
    (:`then`
      (bind (_returnvalue_roll _returnvalue_pitch _returnvalue_yaw) (`KismetMathLibrary.BreakRotator` (`KismetMathLibrary.FindLookAtRotation` (`self.K2_GetActorLocation`) (`self.K2_GetActorLocation` _returnvalue_2))))
      (bind (_returnvalue_roll_2 _returnvalue_pitch_2) (`KismetMathLibrary.BreakRotator` (`KismetMathLibrary.RInterpTo` _returnvalue (`KismetMathLibrary.MakeRotator` 0.0 _returnvalue_pitch _returnvalue_yaw) (`GameplayStatics.GetWorldDeltaSeconds`) 10.0)))
      (`self.K2_SetActorRotation` (`KismetMathLibrary.MakeRotator` 0.0 _returnvalue_pitch_2 (.yaw _returnvalue))))))

(event `self.ReceiveBeginPlay`
  ;[1 1 1] Material Setup
  (bind _returnvalue (`KismetMaterialLibrary.CreateDynamicMaterialInstance` "/Game/VAT-Character-Blueprint/Blueprints/VATBP/VATBP_ANM/StateMachine_Mat/MI_VAT_StateMachineAnimated_Dolphin.MI_VAT_StateMachineAnimated_Dolphin"))
  (bind _output_get (set `self.DynamicMaterial` _returnvalue))
  (`PrimitiveComponent.SetMaterial` (`self.Mesh`) 0 _output_get))

(event `self.ReceiveTick`
  (params (DeltaSeconds :type "Float (single-precision)"))
  ;[1 1 1] Material Setup
  (if (`self.AI?`)
    (`self.AI`)))

(event `InputAxis|Move Forward / Backward`
  (params (AxisValue :type "Float (single-precision)"))
  (bind (_returnvalue_roll _returnvalue_pitch _returnvalue_yaw) (`KismetMathLibrary.BreakRotator` (`self.GetControlRotation`)))
  ;[1 1 1] Dolphin Trajectory
  ;;[1 1 1] Forward Movement
  (bind (_returnvalue_roll_2 _returnvalue_pitch_2 _returnvalue_yaw_2) (`KismetMathLibrary.BreakRotator` (`KismetMathLibrary.FindLookAtRotation` (`self.K2_GetActorLocation`) (`self.K2_GetActorLocation` (stale `AI` _returnvalue_2)))))
  (bind (_returnvalue_roll_3 _returnvalue_pitch_3) (`KismetMathLibrary.BreakRotator` (`KismetMathLibrary.RInterpTo` (`self.K2_GetActorRotation`) (`KismetMathLibrary.MakeRotator` 0.0 _returnvalue_pitch_2 _returnvalue_yaw_2) (`GameplayStatics.GetWorldDeltaSeconds`) 10.0)))
  (`self.AddMovementInput` (`KismetMathLibrary.Vector_GetAbs` (`KismetMathLibrary.GetForwardVector` (`KismetMathLibrary.MakeRotator` _returnvalue_roll _returnvalue_pitch_3 _returnvalue_yaw))) (`KismetMathLibrary.Abs` (`KismetMathLibrary.FClamp` AxisValue 0.0 100.0))))

(event `InputAxis|Move Right / Left`
  (params (AxisValue :type "Float (single-precision)"))
  (bind (_returnvalue_roll _returnvalue_pitch _returnvalue_yaw) (`KismetMathLibrary.BreakRotator` (`self.K2_GetActorRotation`)))
  (bind (_returnvalue_roll_2 _returnvalue_pitch_2 _returnvalue_yaw_2) (`KismetMathLibrary.BreakRotator` (`self.GetControlRotation`)))
  ;[1 1 1] Dolphin Trajectory
  ;;[1 1 1] Rotation
  (bind (_returnvalue_roll_3 _returnvalue_pitch_3 _returnvalue_yaw_3) (`KismetMathLibrary.BreakRotator` (`KismetMathLibrary.FindLookAtRotation` (`self.K2_GetActorLocation`) (`self.K2_GetActorLocation` (stale `AI` _returnvalue_2)))))
  (bind (_returnvalue_roll_4 _returnvalue_pitch_4) (`KismetMathLibrary.BreakRotator` (`KismetMathLibrary.RInterpTo` (`self.K2_GetActorRotation`) (`KismetMathLibrary.MakeRotator` 0.0 _returnvalue_pitch_3 _returnvalue_yaw_3) (`GameplayStatics.GetWorldDeltaSeconds`) 10.0)))
  (`self.AddMovementInput` (`KismetMathLibrary.Normal` (+ (* (`KismetMathLibrary.GetRightVector` (`KismetMathLibrary.MakeRotator` _returnvalue_roll_2 _returnvalue_pitch_4 _returnvalue_yaw_2)) AxisValue) (`KismetMathLibrary.GetForwardVector` (`KismetMathLibrary.MakeRotator` _returnvalue_roll _returnvalue_pitch_4 _returnvalue_yaw)))) (`KismetMathLibrary.Abs` AxisValue)))

(event `InputAxis|Turn Right / Left Mouse`
  (params (AxisValue :type "Float (single-precision)"))
  ;[1 1 1] Dolphin Trajectory
  ;;[1 1 1] Rotation
  (`self.AddControllerYawInput` AxisValue))

(event `InputAxis|Look Up / Down Mouse`
  (params (AxisValue :type "Float (single-precision)"))
  ;[1 1 1] Dolphin Trajectory
  ;;[1 1 1] Rotation
  (`self.AddControllerPitchInput` AxisValue))

(fn `UserConstructionScript`)
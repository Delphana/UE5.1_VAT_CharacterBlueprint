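; Character Blueprint for a common dolphin with player-driven movement and a flag-gated AI move.
; Axis inputs turn the controller and add movement along control/actor-rotation vectors with interpolated pitch; forward input uses absolute direction and scale.
; A Swimming event switches movement to Flying mode.
; Look-at and AI MoveTo targets are the dolphin's own location, AI re-issues every Tick, and a SetActorRotation chain is unconnected.
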(event `AI`
  (`AITask_MoveTo.AIMoveTo` (`AIBlueprintHelperLibrary.GetAIController` self) (`self.K2_GetActorLocation` null) null -1.0 "Default" "Default" false false))

(event `self.ReceiveBeginPlay`)

(event `self.ReceiveTick`
  (params (DeltaSeconds :type "Float (single-precision)"))
  (if (`self.AI?`)
    (`self.AI`)))

(event `InputAxis|Move Forward / Backward`
  (params (AxisValue :type "Float (single-precision)"))
  (bind (_returnvalue_roll _returnvalue_pitch _returnvalue_yaw) (`KismetMathLibrary.BreakRotator` (`self.GetControlRotation`)))
  (bind (_returnvalue_roll_2 _returnvalue_pitch_2 _returnvalue_yaw_2) (`KismetMathLibrary.BreakRotator` (`KismetMathLibrary.FindLookAtRotation` (`self.K2_GetActorLocation`) (`self.K2_GetActorLocation` null))))
  (bind (_returnvalue_roll_3 _returnvalue_pitch_3) (`KismetMathLibrary.BreakRotator` (`KismetMathLibrary.RInterpTo` (`self.K2_GetActorRotation`) (`KismetMathLibrary.MakeRotator` 0.0 _returnvalue_pitch_2 _returnvalue_yaw_2) (`GameplayStatics.GetWorldDeltaSeconds`) 10.0)))
  ;[1 1 1] Dolphin Trajectory
  ;;[1 1 1] Forward Movement
  (`self.AddMovementInput` (`KismetMathLibrary.Vector_GetAbs` (`KismetMathLibrary.GetForwardVector` (`KismetMathLibrary.MakeRotator` _returnvalue_roll _returnvalue_pitch_3 _returnvalue_yaw))) (`KismetMathLibrary.Abs` (`KismetMathLibrary.FClamp` AxisValue 0.0 100.0))))

(event `InputAxis|Move Right / Left`
  (params (AxisValue :type "Float (single-precision)"))
  (bind (_returnvalue_roll _returnvalue_pitch _returnvalue_yaw) (`KismetMathLibrary.BreakRotator` (`self.K2_GetActorRotation`)))
  (bind (_returnvalue_roll_2 _returnvalue_pitch_2 _returnvalue_yaw_2) (`KismetMathLibrary.BreakRotator` (`self.GetControlRotation`)))
  (bind (_returnvalue_roll_3 _returnvalue_pitch_3 _returnvalue_yaw_3) (`KismetMathLibrary.BreakRotator` (`KismetMathLibrary.FindLookAtRotation` (`self.K2_GetActorLocation`) (`self.K2_GetActorLocation` null))))
  (bind (_returnvalue_roll_4 _returnvalue_pitch_4) (`KismetMathLibrary.BreakRotator` (`KismetMathLibrary.RInterpTo` (`self.K2_GetActorRotation`) (`KismetMathLibrary.MakeRotator` 0.0 _returnvalue_pitch_3 _returnvalue_yaw_3) (`GameplayStatics.GetWorldDeltaSeconds`) 10.0)))
  ;[1 1 1] Dolphin Trajectory
  ;;[1 1 1] Rotation
  (`self.AddMovementInput` (`KismetMathLibrary.Normal` (+ (* (`KismetMathLibrary.GetRightVector` (`KismetMathLibrary.MakeRotator` _returnvalue_roll_2 _returnvalue_pitch_4 _returnvalue_yaw_2)) AxisValue) (`KismetMathLibrary.GetForwardVector` (`KismetMathLibrary.MakeRotator` _returnvalue_roll _returnvalue_pitch_4 _returnvalue_yaw)))) (`KismetMathLibrary.Abs` AxisValue)))

(event `InputAxis|Turn Right / Left Mouse`
  (params (AxisValue :type "Float (single-precision)"))
  ;[1 1 1] Dolphin Trajectory
  ;;[1 1 1] Rotation
  (`self.AddControllerYawInput` AxisValue))

(event `InputAxis|Look Up / Down Mouse`
  (params (AxisValue :type "Float (single-precision)"))
  ;[1 1 1] Dolphin Trajectory
  ;;[1 1 1] Rotation
  (`self.AddControllerPitchInput` AxisValue))

(event `Swimming`
  (`CharacterMovementComponent.SetMovementMode` (`self.CharacterMovement`) "MOVE_Flying" 0))

(fn `UserConstructionScript`)
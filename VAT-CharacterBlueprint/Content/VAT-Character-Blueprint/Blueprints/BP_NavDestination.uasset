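; BP_NavDestination is a navigation destination actor that moves along the spline of a referenced SplinePath.
; While FollowSpline is enabled, Tick either plays a timeline scaled by ActorCompletionTime for automatic movement or uses an Alpha value for manual placement.
; Both modes map alpha to distance along the spline, setting world-space location and local-space rotation from that point.
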(event `self.ReceiveBeginPlay`)

(event `FollowSpline`
  (bind _spline (`/Game/VAT-Character-Blueprint/Blueprints/BP_NavSpline.Spline` (`self.SplinePath`)))
  (bind _returnvalue (`SplineComponent.GetSplineLength` _spline))
  (bind _returnvalue_2 (`KismetMathLibrary.Lerp` 0.0 _returnvalue (`self.Alpha`)))
  (if (`self.AutoMove?`)
    (`TimelineComponent.SetPlayRate` (`self.Timeline`) (/ 1.0 (`self.Actor Completion Time`)))
    ;[1 1 1] Destination Moves Automatically
    (bind (_direction _newtrack_0) (`Timeline|Timeline`)
      (:`Update`
        (bind _returnvalue_3 (`KismetMathLibrary.Lerp` 0.0 _returnvalue _newtrack_0))
        (`self.K2_SetActorTransform` (`KismetMathLibrary.MakeTransform` (`SplineComponent.GetLocationAtDistanceAlongSpline` _spline _returnvalue_3 "World") (`SplineComponent.GetRotationAtDistanceAlongSpline` _spline _returnvalue_3 "Local")))))
    (else
      ;[1 1 1] Destination Moves Manually (controlled by alpha)
      (`self.K2_SetActorTransform` (`KismetMathLibrary.MakeTransform` (`SplineComponent.GetLocationAtDistanceAlongSpline` _spline _returnvalue_2 "World") (`SplineComponent.GetRotationAtDistanceAlongSpline` _spline _returnvalue_2 "Local"))))))

(event `self.ReceiveTick`
  (params (DeltaSeconds :type "Float (single-precision)"))
  (if (`self.FollowSpline?`)
    (`self.FollowSpline`)))

(fn `UserConstructionScript`)
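; BP_DolphinSpawn is a placement Blueprint that lays out grids of child actors, presumably dolphins, from an array of actor classes.
; The Construction Script sizes parallel count, spacing and transform arrays to match the class array.
; For each entry it adds Child Actor Components on an X-by-Y grid, using integer divide and modulo for offsets from that entry's transform.
; The Event Graph has no active logic.
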(fn `UserConstructionScript`
  (bind _num (`self.Num`))
  (bind _actor (`self.Actor`))
  (bind _returnvalue (`KismetArrayLibrary.Array_Length` (`self.Actor`)))
  (`KismetArrayLibrary.Array_Resize` _num _returnvalue)
  (for (_ _array_index) _num
    (`KismetArrayLibrary.Array_Resize` (`self.Space_X`) _returnvalue)
    (`KismetArrayLibrary.Array_Resize` (`self.Space_Y`) _returnvalue)
    (`KismetArrayLibrary.Array_Resize` (`self.Y`) _returnvalue)
    (`KismetArrayLibrary.Array_Resize` (`self.X`) _returnvalue)
    (`KismetArrayLibrary.Array_Resize` (`self.SpawnedTransform`) _returnvalue)
    (bind _output (`|GetArrayItem` (`self.Y`) _array_index))
    (for _index (range (* (`|GetArrayItem` (`self.X`) _array_index) _output))
      (bind (_output_location _output_rotation _output_scale) (`KismetMathLibrary.BreakTransform` (`|GetArrayItem` (`self.SpawnedTransform`) _array_index)))
      (bind _returnvalue_2 (`AddComponent|NODE_AddChildActorComponent-0` :`RelativeTransform` (`KismetMathLibrary.MakeTransform` (+ (`KismetMathLibrary.MakeVector` (* (/ _index _output) (`|GetArrayItem` (`self.Space_X`) _array_index)) (* (mod _index _output) (`|GetArrayItem` (`self.Space_Y`) _array_index))) _output_location) _output_rotation _output_scale)))
      (`ChildActorComponent.SetChildActorClass` _returnvalue_2 (`|GetArrayItem` _actor _array_index))
      (for _ _actor
        _))))